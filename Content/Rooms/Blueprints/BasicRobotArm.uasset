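; Robot arm actor with yaw/pitch joints and a two-finger gripper, driven by command parameters read from GameInstanceTCPServer.
; Events rotate joints by the received angle, while base yaw and pitch also support velocity mode via looping 20 Hz timers.
; Grip open/close moves both fingers with sweep; reset restores the pose but clears only the yaw timer.
; Helpers expose gripper midpoint, comma-joined vector text and a camera render target (marked TODO).
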(event `RobotArmReset`
  (`SceneComponent.K2_SetRelativeRotation` :`self` (`self.BaseYaw`))
  (`SceneComponent.K2_SetRelativeRotation` (`self.BasePitch`) (struct :`Pitch` 90.0) false false)
  (`SceneComponent.K2_SetRelativeRotation` (`self.ElbowPitch`) (struct :`Pitch` 90.0) false false)
  (`SceneComponent.K2_SetRelativeRotation` :`self` (`self.WristYaw`))
  (`SceneComponent.K2_SetRelativeRotation` (`self.WristPitch`) (struct :`Pitch` 90.0) false false)
  (`SceneComponent.K2_SetRelativeLocation` (`self.Grip1`) (85.0 0.0 -40.0) false false)
  (`SceneComponent.K2_SetRelativeLocation` (`self.Grip2`) (85.0 0.0 40.0) false false)
  (`KismetSystemLibrary.K2_ClearAndInvalidateTimerHandle` (`self.baseYawEvt`)))

(event `self.ReceiveBeginPlay`
  (`self.RobotArmReset`))

(event `RotateBaseYaw`
  (bind _cmdparameter (`self.GetCmdFloatParameter`))
  (`SceneComponent.K2_AddRelativeRotation` (`self.BaseYaw`) (`KismetMathLibrary.MakeRotator` 0.0 0.0 _cmdparameter) false false))

(event `RotateBasePitch`
  (bind _basepitch (`self.BasePitch`))
  (bind _cmdparameter (`self.GetCmdFloatParameter`))
  (`SceneComponent.K2_AddWorldRotation` _basepitch (`KismetMathLibrary.RotatorFromAxisAndAngle` (`SceneComponent.GetUpVector` _basepitch) _cmdparameter) false false))

(event `RotateElbowPitch`
  (bind _elbowpitch (`self.ElbowPitch`))
  (bind _cmdparameter (`self.GetCmdFloatParameter`))
  (`SceneComponent.K2_AddWorldRotation` _elbowpitch (`KismetMathLibrary.RotatorFromAxisAndAngle` (`SceneComponent.GetUpVector` _elbowpitch) _cmdparameter) false false))

(event `BaseYawVelocity`
  (bind _cmdparameter (`self.GetCmdFloatParameter`))
  (set `self.BaseYawVelValue` _cmdparameter)
  (if (>= (`KismetMathLibrary.Abs` _cmdparameter) 0.01)
    (bind _returnvalue (`KismetSystemLibrary.K2_SetTimerDelegate` (delegate `BaseYawVel_evt`) 0.05 true))
    (set `self.baseYawEvt` _returnvalue)
    (else
      (`KismetSystemLibrary.K2_ClearAndInvalidateTimerHandle` (`self.baseYawEvt`)))))

(event `RotateWristYaw`
  (bind _wristyaw (`self.WristYaw`))
  (bind _cmdparameter (`self.GetCmdFloatParameter`))
  (`SceneComponent.K2_AddWorldRotation` _wristyaw (`KismetMathLibrary.RotatorFromAxisAndAngle` (`SceneComponent.GetUpVector` _wristyaw) _cmdparameter) false false))

(event `BaseYawVel_evt`
  (`SceneComponent.K2_AddRelativeRotation` (`self.BaseYaw`) (`KismetMathLibrary.MakeRotator` 0.0 0.0 (/ (`self.BaseYawVelValue`) 20.0)) false false))

(event `RotateWristPitch`
  (bind _wristpitch (`self.WristPitch`))
  (bind _cmdparameter (`self.GetCmdFloatParameter`))
  (`SceneComponent.K2_AddWorldRotation` _wristpitch (`KismetMathLibrary.RotatorFromAxisAndAngle` (`SceneComponent.GetUpVector` _wristpitch) _cmdparameter) false false))

(event `BasePitchVelocity`
  (bind _cmdparameter (`self.GetCmdFloatParameter`))
  (set `self.BasePitchVelValue` _cmdparameter)
  (if (>= (`KismetMathLibrary.Abs` _cmdparameter) 0.01)
    (bind _returnvalue (`KismetSystemLibrary.K2_SetTimerDelegate` (delegate `BasePitchVel_evt`) 0.05 true))
    (set `self.BasePitchEvt` _returnvalue)
    (else
      (`KismetSystemLibrary.K2_ClearAndInvalidateTimerHandle` (`self.BasePitchEvt`)))))

(event `OpenGrip`
  (`SceneComponent.K2_SetRelativeLocation` (`self.Grip1`) (85.0 0.0 -40.0) true false)
  (`SceneComponent.K2_SetRelativeLocation` (`self.Grip2`) (85.0 0.0 40.0) true false))

(event `BasePitchVel_evt`
  (bind _basepitch (`self.BasePitch`))
  (`SceneComponent.K2_AddWorldRotation` _basepitch (`KismetMathLibrary.RotatorFromAxisAndAngle` (`SceneComponent.GetUpVector` _basepitch) (/ (`self.BasePitchVelValue`) 20.0)) false false))

(event `CloseGrip`
  (`SceneComponent.K2_SetRelativeLocation` (`self.Grip1`) (85.0 0.0 -5.0) true false)
  (`SceneComponent.K2_SetRelativeLocation` (`self.Grip2`) (85.0 0.0 5.0) true false))

(fn `GetCamImage`
  (returns (textureOut :type "TextureRenderTarget2D Object Reference"))
  (cast `/Game/Rooms/Blueprints/CameraSensor` (`ChildActorComponent.ChildActor` (`self.cameraSensor`))
    (:`then`
      ;[1 1 1] TODO : a corriger!
      (return "/Game/Rooms/Blueprints/CamSensor_RenderTarget2D.CamSensor_RenderTarget2D"))
    (:`CastFailed`
      (`KismetSystemLibrary.PrintString` "Cast Error : cannot get Cam Image")
      (return "/Game/Rooms/Blueprints/CamSensor_RenderTarget2D.CamSensor_RenderTarget2D"))))

(fn `GetCmdFloatParameter`
  (returns (CmdParameter :type "Float (double-precision)"))
  (bind _asgame_instance_tcpserver (cast `/Game/MainSystem/GameInstanceTCPServer` (`GameplayStatics.GetGameInstance`)))
  (return (`KismetStringLibrary.Conv_StringToDouble` (`/Game/MainSystem/GameInstanceTCPServer.cmdParams` _asgame_instance_tcpserver))))

(fn `GetCmdFloatParameters`
  (returns (CmdParameters :type "Array of Float (double-precision)"))
  (locals (params :type "Array of Float (double-precision)") (loopOn :type Boolean :default true) (strToSplit :type String))
  (bind (_lefts _rights _returnvalue) (`KismetStringLibrary.Split` (`local.strToSplit`) " "))
  (bind _asgame_instance_tcpserver (cast `/Game/MainSystem/GameInstanceTCPServer` (`GameplayStatics.GetGameInstance`)))
  (set `local.strToSplit` (`/Game/MainSystem/GameInstanceTCPServer.cmdParams` _asgame_instance_tcpserver))
  (while (`local.loopOn`)
    (`KismetArrayLibrary.Array_Add` (`local.params`) (`KismetStringLibrary.Conv_StringToDouble` _lefts))
    (if _returnvalue
      (set `local.strToSplit` _rights)
      (else
        (set `local.loopOn` false))))
  (return (`local.params`)))

(fn `GetGripperPos`
  (returns (pos :type "Vector Structure"))
  (return (/ (+ (`SceneComponent.K2_GetComponentLocation` (`self.Grip1`)) (`SceneComponent.K2_GetComponentLocation` (`self.Grip2`))) 2.0)))

(fn `UserConstructionScript`)

(fn `VectorToJson`
  (params (vec :type "Vector Structure"))
  (returns (json :type String))
  (return (`KismetStringLibrary.Concat_StrStr` (`KismetStringLibrary.Conv_DoubleToString` vec_X) "," (`KismetStringLibrary.Conv_DoubleToString` vec_Y) "," (`KismetStringLibrary.Conv_DoubleToString` vec_Z))))